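; BP_Floor is a floor actor with X/Y grid numbers that takes over the player's view when a BP_Operator enters its Box trigger.
; On overlap, it switches player controller 0's view target to itself and writes its floor numbers into the operator's CurrentX and CurrentY.
; It prints the new Y/X position as debug text, or "Hello" for any other overlapping actor.
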(event `self.Box.OnComponentBeginOverlap`
  (params (OverlappedComponent :type "PrimitiveComponent Object Reference") (OtherActor :type "Actor Object Reference") (OtherComp :type "PrimitiveComponent Object Reference") (OtherBodyIndex :type Integer) (bFromSweep :type Boolean) (SweepResult :type "HitResult Structure (by ref)"))
  (bind _asbp_operator (cast `/Game/Blueprint/BP_Operator` OtherActor)
    (:`then`
      (`PlayerController.SetViewTargetWithBlend` (`GameplayStatics.GetPlayerController` 0) self 0.0 "VTBlend_Linear" 0.0 false)
      (bind _output_get (set `/Game/Blueprint/BP_Operator.CurrentY` (`self.FloorNumberY`) _asbp_operator))
      (bind _output_get_2 (set `/Game/Blueprint/BP_Operator.CurrentX` (`self.FloorNumberX`) _asbp_operator))
      (`KismetSystemLibrary.PrintString` (`KismetStringLibrary.Concat_StrStr` (`KismetStringLibrary.Conv_IntToString` _output_get) " / " (`KismetStringLibrary.Conv_IntToString` _output_get_2))))
    (:`CastFailed`
      (`KismetSystemLibrary.PrintString` "Hello"))))

(fn `UserConstructionScript`)