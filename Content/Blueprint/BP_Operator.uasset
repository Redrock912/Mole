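; BP_Operator is a player-controlled pawn blueprint that turns and moves in the direction of the MoveForward and MoveRight input axes.
; While either axis is non-zero, Tick builds a world-space rotation from both values and sets it as the control rotation.
; It then adds full-scale movement along the player controller's forward vector.
; The axis events are empty, and conventional per-axis movement nodes remain unconnected.
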(event `self.ReceiveTick`
  (params (DeltaSeconds :type "Float (single-precision)"))
  (if (or (!= (`self.GetInputAxisValue`) 0.0) (!= (`self.GetInputAxisValue`) 0.0))
    (`Controller.SetControlRotation` (`GameplayStatics.GetPlayerController` 0) (`KismetMathLibrary.MakeRotFromX` (`KismetMathLibrary.MakeVector` (`self.GetInputAxisValue`) (`self.GetInputAxisValue`))))
    (`self.AddMovementInput` (`self.GetActorForwardVector` (`GameplayStatics.GetPlayerController` 0)))))

(event `InputAxis|MoveForward`
  (params (AxisValue :type "Float (single-precision)")))

(event `InputAxis|MoveRight`
  (params (AxisValue :type "Float (single-precision)")))

(fn `UserConstructionScript`)